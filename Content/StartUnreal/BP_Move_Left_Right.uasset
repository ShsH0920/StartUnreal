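; Actor Blueprint that slides its Sphere component back and forth along the relative X axis.
; Each Tick offsets the sphere by delta time times Speed, with the IsRightMove flag selecting the direction.
; The flag flips when the sphere's relative X passes a hardcoded upper or lower bound, producing a continuous ping-pong motion.
; BeginPlay, overlap and construction logic are empty, and IsUpMove is unused.
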(event `self.ReceiveTick`
  (params (DeltaSeconds :type "Float (single-precision)"))
  (bind _sphere (`self.Sphere`))
  (bind _returnvalue (* DeltaSeconds (`self.Speed`)))
  (bind _relativelocation_x (`KismetMathLibrary.BreakVector` (`SceneComponent.RelativeLocation` _sphere)))
  (bind _relativelocation_x_2 (`KismetMathLibrary.BreakVector` (`SceneComponent.RelativeLocation` _sphere)))
  (if (`self.isRightMove`)
    (`SceneComponent.K2_AddRelativeLocation` _sphere (`KismetMathLibrary.MakeVector` _returnvalue) false false)
    (if (> _relativelocation_x 100.0)
      (set `self.isRightMove` false))
    (else
      (bind _result (`/Engine/EditorBlueprintResources/StandardMacros.NegateFloat` _returnvalue)
        (:`  `
          (`SceneComponent.K2_AddRelativeLocation` _sphere (`KismetMathLibrary.MakeVector` _result) false false)
          (if (<= _relativelocation_x_2 0.0)
            (set `self.isRightMove` true)))))))

(fn `UserConstructionScript`)