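; BP_Pawn is a test pawn in StartUnreal with axis-driven movement, look input and debug prints.
; Move axes offset the actor along its forward and right vectors, unscaled by delta time, with a larger sideways step.
; LookUp feeds controller yaw and LookRight feeds pitch, opposite to their names.
; Tick calls ShowTimeSet, printing accumulated seconds modulo 60 whenever they change; NewFunction0 is never called.
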(event `self.ReceiveBeginPlay`
  (`KismetSystemLibrary.PrintString` "BeginPlay"))

(event `InputAction|EnterInput`
  (params (Key :type "Key Structure"))
  (:`Pressed`
    (`KismetSystemLibrary.PrintString` "Enter_Pressed")))

(event `self.ReceiveTick`
  (params (DeltaSeconds :type "Float (single-precision)"))
  (`self.Show Time Set` DeltaSeconds))

(event `Key|W`
  (params (Key :type "Key Structure"))
  (:`Pressed`
    (`KismetSystemLibrary.PrintString` "W_Pressed")))

(event `InputAxis|Move Foward`
  (params (AxisValue :type "Float (single-precision)"))
  ;[0.8409 0.602 1] 앞쪽으로 움직임
  (`self.K2_AddActorWorldOffset` (* (`self.GetActorForwardVector`) (* AxisValue 10.0))))

(event `InputAxis|Move Right`
  (params (AxisValue :type "Float (single-precision)"))
  ;[1 1 1] 옆으로 움직임
  (`self.K2_AddActorWorldOffset` (* (`self.GetActorRightVector`) (* AxisValue 100.0))))

(event `InputAxis|LookUp`
  (params (AxisValue :type "Float (single-precision)"))
  ;[1 1 1] 위아래를 보기
  (`self.AddControllerYawInput` AxisValue))

(event `InputAxis|LookRight`
  (params (AxisValue :type "Float (single-precision)"))
  ;[1 1 1] 옆을 보기
  (`self.AddControllerPitchInput` AxisValue))

(fn `NewFunction_0`
  (params (A :type "Float (double-precision)"))
  (bind _output_get (set `self.TotalDeltaSecond` (+ A (`self.TotalDeltaSecond`))))
  (`KismetSystemLibrary.PrintString` (`KismetStringLibrary.Concat_StrStr` "TDelta Seconds -" (`KismetStringLibrary.Conv_DoubleToString` _output_get))))

(fn `Show Time Set`
  (params (DeltaSeconds :type "Float (double-precision)"))
  (bind _output_get (set `self.TotalDeltaSecond` (+ DeltaSeconds (`self.TotalDeltaSecond`))))
  (bind _returnvalue (`KismetMathLibrary.FFloor` (mod _output_get 60.0)))
  (if (not (== (`self.BeforeInt`) _returnvalue))
    (`KismetSystemLibrary.PrintString` (`KismetStringLibrary.Concat_StrStr` "TDelta Seconds :" (`KismetStringLibrary.Conv_IntToString` _returnvalue)) true true (struct :`G` 0.66 :`B` 1.0 :`A` 1.0) 1.0)
    (set `self.BeforeInt` _returnvalue)))

(fn `UserConstructionScript`)